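; SkeeballGame_BP is a skeeball scoring actor with overlap components for holes worth 20, 30, 50 and 100 points.
; Each overlap adds its value to Points and compares the sum with MaxPoints as 64-bit integers, calling DestroyActor when they differ.
; The sum is never written back to Points, and an exact match triggers nothing.
; BeginPlay, Tick and the construction script are empty.
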(event OnComponentBeginOverlap(20points)
  (params (OverlappedComponent :type Primitive%20Component%20Object%20Reference) (OtherActor :type Actor%20Object%20Reference) (OtherComp :type Primitive%20Component%20Object%20Reference) (OtherBodyIndex :type Integer) (bFromSweep :type Boolean) (SweepResult :type Hit%20Result%20Structure%20%28by%20ref%29))
  (if (not (== (Class|KismetMathLibrary|ToInt64(Integer) (+ (Variables|Default|GetPoints%20) 20)) (Class|KismetMathLibrary|ToInt64(Integer) (Variables|Default|GetMaxPoints))))
    (Actor|DestroyActor)))

(event OnComponentBeginOverlap(30points)
  (params (OverlappedComponent :type Primitive%20Component%20Object%20Reference) (OtherActor :type Actor%20Object%20Reference) (OtherComp :type Primitive%20Component%20Object%20Reference) (OtherBodyIndex :type Integer) (bFromSweep :type Boolean) (SweepResult :type Hit%20Result%20Structure%20%28by%20ref%29))
  (if (not (== (Class|KismetMathLibrary|ToInt64(Integer) (+ (Variables|Default|GetPoints%20) 30)) (Class|KismetMathLibrary|ToInt64(Integer) (Variables|Default|GetMaxPoints))))
    (Actor|DestroyActor)))

(event OnComponentBeginOverlap(50points)
  (params (OverlappedComponent :type Primitive%20Component%20Object%20Reference) (OtherActor :type Actor%20Object%20Reference) (OtherComp :type Primitive%20Component%20Object%20Reference) (OtherBodyIndex :type Integer) (bFromSweep :type Boolean) (SweepResult :type Hit%20Result%20Structure%20%28by%20ref%29))
  (if (not (== (Class|KismetMathLibrary|ToInt64(Integer) (+ (Variables|Default|GetPoints%20) 50)) (Class|KismetMathLibrary|ToInt64(Integer) (Variables|Default|GetMaxPoints))))
    (Actor|DestroyActor)))

(event OnComponentBeginOverlap(100points)
  (params (OverlappedComponent :type Primitive%20Component%20Object%20Reference) (OtherActor :type Actor%20Object%20Reference) (OtherComp :type Primitive%20Component%20Object%20Reference) (OtherBodyIndex :type Integer) (bFromSweep :type Boolean) (SweepResult :type Hit%20Result%20Structure%20%28by%20ref%29))
  (if (not (== (Class|KismetMathLibrary|ToInt64(Integer) (+ (Variables|Default|GetPoints%20) 100)) (Class|KismetMathLibrary|ToInt64(Integer) (Variables|Default|GetMaxPoints))))
    (Actor|DestroyActor)))

(event EventBeginPlay)

(event Collision|EventActorBeginOverlap
  (params (OtherActor :type Actor%20Object%20Reference)))

(event EventTick
  (params (DeltaSeconds :type Float%20%28single-precision%29)))

(fn ConstructionScript)